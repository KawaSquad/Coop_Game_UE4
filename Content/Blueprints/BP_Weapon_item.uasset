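; BP_Weapon_item is a rotating weapon pickup that gives a gun to a character who touches it.
; On BeginPlay it takes its skeletal mesh from WeaponType, and Tick spins it around yaw at RotationSpeed.
; When a BP_Character overlaps its sphere, it optionally destroys itself if AutoDestroy is set, then calls GiveThisMenAGun with the WeaponType's weapon class.
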(event `self.ReceiveTick`
  (params (DeltaSeconds :type "Float (single-precision)"))
  (`self.K2_AddActorLocalRotation` (`KismetMathLibrary.MakeRotator` 0.0 0.0 (* DeltaSeconds (`self.RotationSpeed`)))))

(event `self.Sphere.OnComponentBeginOverlap`
  (params (OverlappedComponent :type "PrimitiveComponent Object Reference") (OtherActor :type "Actor Object Reference") (OtherComp :type "PrimitiveComponent Object Reference") (OtherBodyIndex :type Integer) (bFromSweep :type Boolean) (SweepResult :type "HitResult Structure (by ref)"))
  (bind _asbp_character (cast `/Game/Blueprints/BP_Character` OtherActor))
  (if (`self.AutoDestroy`)
    (`self.K2_DestroyActor`))
  (`/Game/Blueprints/BP_Character.GiveThisMenAGun` _asbp_character (`.WeaponClass_2_62220663472751AC4ADC889C56EBC7C3` (break `/Game/Blueprints/WeaponType` (`self.Weapon_Type`)))))

(event `self.ReceiveBeginPlay`
  (`SkinnedMeshComponent.SetSkinnedAssetAndUpdate` (`self.MeshComp`) (`.MeshComp_5_22DC54B547BF4ED9090FA49EA181AD13` (break `/Game/Blueprints/WeaponType` (`self.Weapon_Type`))) true))

(fn `UserConstructionScript`)